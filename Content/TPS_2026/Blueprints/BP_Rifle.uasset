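; BP_Rifle is an automatic rifle actor for a third-person shooter that spawns bullets while the trigger is held.
; StartFire and EndFire toggle IsFiring, and Tick accumulates time to call Fire whenever the FireRate interval has elapsed.
; Fire spawns a BP_Bullet at the mesh's Muzzle_Socket, rotated toward AimLocation, which is not set within this Blueprint.
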(event EventBeginPlay)

(event Collision|EventActorBeginOverlap
  (params (OtherActor :type Actor%20Object%20Reference)))

(event EventTick
  (params (DeltaSeconds :type Float%20%28single-precision%29))
  (Variables|Default|SetFireRateDelta (+ DeltaSeconds (Variables|Default|GetFireRateDelta)))
  (if (and (Variables|Default|GetisFiring) (>= (Variables|Default|GetFireRateDelta) (Variables|Default|GetFireRate)))
    (Variables|Default|SetFireRateDelta 0.0)
    (CallFunction|Fire)))

(fn ConstructionScript)

(fn Fire
  (bind _riflemesh (Variables|Default|GetRifleMesh))
  (bind _returnvalue (Transformation|GetSocketTransform _riflemesh "Muzzle_Socket" "RTS_World"))
  (Game|SpawnActorfromClass "/Game/TPS_2026/Blueprints/BP_Bullet.BP_Bullet_C" (Math|Transform|MakeTransform (.location _returnvalue) (Math|Rotator|FindLookatRotation (.location _returnvalue) (Variables|Default|GetaimLocation)) (.scale _returnvalue)) "Undefined" "MultiplyWithRoot" 0 0))

(fn StartFire
  (Variables|Default|SetisFiring true))

(fn EndFire
  (Variables|Default|SetisFiring false))